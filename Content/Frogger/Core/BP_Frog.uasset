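; BP_Frog is the Frogger frog actor, colored with the color saved in BP_GameInstance.
; BeginPlay binds an event to color changes on every sample in the WBP_ColorPicker widget, then applies the saved color.
; SetActorColor writes the SkinColor parameter through a dynamic material on the Cube mesh.
; It also destroys the PlayerTracker widget component in the Menu level, or tints that widget to match in other levels.
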(event EventBeginPlay
  (bind _foundwidgets (Widget|GetAllWidgetsOfClass "/Game/Frogger/Art/UI/Lobby/WBP_ColorPicker.WBP_ColorPicker_C" false))
  (CallFunction|BindtoColorPicked (Utilities|Array|Get(acopy) _foundwidgets))
  (bind _asbp_game_instance (Utilities|Casting|CastToBP_GameInstance (Game|GetGameInstance)))
  (CallFunction|SetActorColor (Variables|/Game/Frogger/Core/BP_GameInstance.BP_GameInstance_C|GetColor _asbp_game_instance)))

(fn ConstructionScript)

(fn SetActorColor
  (params (Color :type Linear%20Color%20Structure))
  (bind _cube (Variables|Default|GetCube))
  (Development|PrintString "Hello")
  (bind _returnvalue (Rendering|Material|CreateDynamicMaterialInstance _cube 0 (Rendering|Material|GetMaterial _cube 0) "None" :!class /Script/Engine.PrimitiveComponent))
  (Rendering|Material|SetVectorParameterValue _returnvalue "SkinColor" Color :!class /Script/Engine.MaterialInstanceDynamic)
  (bind _returnvalue_2 (Game|GetCurrentLevelName true))
  (if (Utilities|Enum|Equal(Enum) _returnvalue_2 "Menu")
    (Components|DestroyComponent (Variables|Default|GetPlayerTracker))
    (else
      (bind _aswbp_player_tracker (Utilities|Casting|CastToWBP_PlayerTracker (UserInterface|GetUserWidgetObject (Variables|Default|GetPlayerTracker))))
      (Default|SetPlayerTrackerColor _aswbp_player_tracker Color))))

(fn BindtoColorPicked
  (params (ColorPicker :type WBP%20Color%20Picker%20Object%20Reference))
  (for _array_element (Variables|/Game/Frogger/Art/UI/Lobby/WBP_ColorPicker.WBP_ColorPicker_C|GetAllSamples ColorPicker)
    (bind _aswbp_color_sample (Utilities|Casting|CastToWBP_ColorSample _array_element))
    (EventDispatchers|BindEventtoOnColorChanged _aswbp_color_sample (EventDispatchers|CreateEvent :!event SetActorColor))))