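; BP_LobbyGameMode is the Frogger lobby game mode that handles players joining and leaving.
; After a short delay on login, it asks the new player's controller through client calls for a color and name.
; On logout, it has the game state multicast a log event with the leaving player's name and an updated player status with the player count.
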(event EventOnLogout
  (params (ExitingController :type Controller%20Object%20Reference))
  (bind _asbp_frogger_player_controller (Utilities|Casting|CastToBP_FroggerPlayerController ExitingController))
  (bind _asbp_frogger_player_state (Utilities|Casting|CastToBP_FroggerPlayerState (Variables|/Script/Engine.Controller|GetPlayerState _asbp_frogger_player_controller)))
  (bind _asbp_frogger_game_state (Utilities|Casting|CastToBP_FroggerGameState (Game|GetGameState)))
  (Default|MulticastLogEvent _asbp_frogger_game_state (Variables|/Game/Frogger/Core/BP_FroggerPlayerState.BP_FroggerPlayerState_C|GetPlayerName _asbp_frogger_player_state) "NewEnumerator1")
  (Default|MulticastUpdatePlayerStatus _asbp_frogger_game_state (Variables|Default|GetNumPlayers) 0 true))

(event EventPostLogin
  (params (NewPlayer :type Player%20Controller%20Object%20Reference))
  (Utilities|FlowControl|Delay 0.2)
  (bind _asbp_frogger_player_controller (Utilities|Casting|CastToBP_FroggerPlayerController NewPlayer))
  (Default|ClientAskforColor _asbp_frogger_player_controller)
  (Default|ClientGetName _asbp_frogger_player_controller))

(fn ConstructionScript)