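; BP_WaterObject is a Frogger actor pairing a mesh with a Niagara emitter that produces foam.
; On BeginPlay it sets the emitter's EmitterSize vector from the Y extent of the mesh's bounds.
; Each tick it feeds the mesh's physics X velocity into the emitter's FoamVelocity parameter, so the effect follows the object's motion.
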(event EventBeginPlay
  (CallFunction|SetParticlesParameters))

(event EventTick
  (params (DeltaSeconds :type Float%20%28single-precision%29))
  (bind _returnvalue (Physics|GetPhysicsLinearVelocity (Variables|Default|GetMesh) "None"))
  (Effects|Components|ParticleSystem|SetFloatParameter (Variables|Default|GetNiagaraEmitter) "FoamVelocity" (.x _returnvalue)))

(fn ConstructionScript)

(fn SetParticlesParameters
  (Effects|Components|ParticleSystem|SetVectorParameter (Variables|Default|GetNiagaraEmitter) "EmitterSize" (Math|Vector|MakeVector 0.0 (.y (.BoxExtent (Collision|GetComponentBounds (Variables|Default|GetMesh)))) 0.0)))