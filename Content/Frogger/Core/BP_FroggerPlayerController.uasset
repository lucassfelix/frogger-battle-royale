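; Player controller for Frogger that negotiates each player's color between client and server.
; The local color lives in the GameInstance, with getter and setter helpers, and is sent to the server on request.
; Server events pass join and availability checks to the GameState, which tracks picked colors.
; Client events store assigned colors or update the color picker widget, though the unavailable-color handler only looks up the widget.
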(event Custom|Server_SendColor
  (params (PlayerController :type BP%20Frogger%20Player%20Controller%20Object%20Reference) (MyColor :type Linear%20Color%20Structure))
  (bind _asbp_frogger_game_state (Utilities|Casting|CastToBP_FroggerGameState (Game|GetGameState)))
  (Default|OnPlayerEntered _asbp_frogger_game_state PlayerController MyColor))

(event Custom|Client_AskForColor
  (bind _asbp_game_instance (Utilities|Casting|CastToBP_GameInstance (Game|GetGameInstance)))
  (bind _asbp_frogger_player_controller (Utilities|Casting|CastToBP_FroggerPlayerController (Game|GetPlayerController 0)))
  (CallFunction|ServerSendColor _asbp_frogger_player_controller (Variables|/Game/Frogger/Core/BP_GameInstance.BP_GameInstance_C|GetColor _asbp_game_instance)))

(event Custom|Server_CheckColorAvailability
  (params (NewColor :type Linear%20Color%20Structure%20%28by%20ref%29) (OldColor :type Linear%20Color%20Structure%20%28by%20ref%29) (PlayerController :type BP%20Frogger%20Player%20Controller%20Object%20Reference))
  (bind _asbp_frogger_game_state (Utilities|Casting|CastToBP_FroggerGameState (Game|GetGameState)))
  (if (Utilities|Set|Contains (Variables|/Game/Frogger/Core/BP_FroggerGameState.BP_FroggerGameState_C|GetPickedColors _asbp_frogger_game_state) NewColor)
    (Default|OnColorUnavaiable _asbp_frogger_game_state PlayerController NewColor)
    (else
      (Default|OnColorAvailable _asbp_frogger_game_state))))

(event Custom|Client_OnColorUnavailable
  (params (Color :type Linear%20Color%20Structure%20%28by%20ref%29))
  (bind _foundwidgets (Widget|GetAllWidgetsOfClass "/Game/Frogger/Art/UI/Lobby/WBP_ColorPicker.WBP_ColorPicker_C" false))
  (if (Utilities|Array|IsEmpty _foundwidgets)
    _))

(event Custom|Client_OnColorAvailable
  (params (Color :type Linear%20Color%20Structure%20%28by%20ref%29))
  (bind _foundwidgets (Widget|GetAllWidgetsOfClass "/Game/Frogger/Art/UI/Lobby/WBP_ColorPicker.WBP_ColorPicker_C" false))
  (if (not (Utilities|Array|IsEmpty _foundwidgets))
    (Default|SetSelectedColor (Utilities|Array|Get(acopy) _foundwidgets) Color false)))

(event Custom|Client_SetColor
  (params (Color :type Linear%20Color%20Structure))
  (bind _asbp_game_instance (Utilities|Casting|CastToBP_GameInstance (Game|GetGameInstance)))
  (Variables|/Game/Frogger/Core/BP_GameInstance.BP_GameInstance_C|SetColor _asbp_game_instance Color)
  (bind _foundwidgets (Widget|GetAllWidgetsOfClass "/Game/Frogger/Art/UI/Lobby/WBP_ColorPicker.WBP_ColorPicker_C" false))
  (if (not (Utilities|Array|IsEmpty _foundwidgets))
    (Default|SetSelectedColor (Utilities|Array|Get(acopy) _foundwidgets) Color false)))

(fn ConstructionScript)

(fn GetColor
  (bind _asbp_game_instance (Utilities|Casting|CastToBP_GameInstance (Game|GetGameInstance)))
  (return (Variables|/Game/Frogger/Core/BP_GameInstance.BP_GameInstance_C|GetColor _asbp_game_instance)))

(fn SetColor
  (params (NewColor :type Linear%20Color%20Structure))
  (bind _asbp_game_instance (Utilities|Casting|CastToBP_GameInstance (Game|GetGameInstance)))
  (Variables|/Game/Frogger/Core/BP_GameInstance.BP_GameInstance_C|SetColor _asbp_game_instance NewColor))