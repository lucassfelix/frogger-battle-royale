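; Game state for the Frogger multiplayer lobby, coordinating player names, unique colors and ready status.
; On entry it keeps a player's color or assigns the first free one, then multicasts taken colors to the lobby color picker.
; Login and status multicasts fire dispatchers for listeners.
; The server counts ready players and travels to the game when all are ready, leaving an older multicast open-level path unused.
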(event Custom|OnPlayerEntered
  (params (NewPlayerController :type BP%20Frogger%20Player%20Controller%20Object%20Reference) (MyColor :type Linear%20Color%20Structure))
  (if (Utilities|Set|Contains (Variables|Default|GetPickedColors) MyColor)
    (bind _array_element (Utilities|Array|ForEachLoopwithBreak (CallFunction|GetPlayerColorsArray) :!label _label)
      (:LoopBody
        (if (not (Utilities|Set|Contains (Variables|Default|GetPickedColors) _array_element))
          (Default|ClientSetColor NewPlayerController _array_element)
          (Utilities|Set|Add (Variables|Default|GetPickedColors) _array_element)
          (goto _label Break)))
      (:Completed
        (bind _result (Utilities|Set|ToArray (Variables|Default|GetPickedColors) :!label _label_2))
        (CallFunction|MulticastBlockedColors _result)))
    (else
      (Utilities|Set|Add (Variables|Default|GetPickedColors) MyColor)
      (Default|ClientSetColor NewPlayerController MyColor)
      (goto _label_2))))

(event Custom|Server_PlayerLoginMessages
  (params (PlayerName :type Text))
  (CallFunction|MulticastLogEvent PlayerName "NewEnumerator0")
  (CallFunction|MulticastUpdatePlayerStatus (Class|GameplayStatics|GetNumPlayerControllers) 0 true))

(event Custom|UpdateReadyCount
  (params (IsReady :type Boolean))
  (bind _returnvalue (Class|GameplayStatics|GetNumPlayerControllers))
  (bind _numready (Variables|Default|GetNumReady))
  (Networking|SwitchHasAuthority
    (:Authority
      (if IsReady
        (Math|Integer|IncrementInt _numready
          (:%20%20
            _))
        (else
          (Math|Integer|DecrementInt _numready
            (:%20%20
              _))))
      (CallFunction|MulticastUpdatePlayerStatus _returnvalue _numready false)
      (if (== (Variables|Default|GetNumReady) _returnvalue)
        (CallFunction|StartMatch)))))

(event Custom|Multicast_BlockedColors
  (params (BlockedColors :type Array%20of%20Linear%20Color%20Structures))
  (bind _asbp_lobby_hud (Utilities|Casting|CastToBP_LobbyHUD (HUD|GetHUD (Game|GetPlayerController 0))))
  (Utilities|IsValid (Variables|/Game/Frogger/Art/UI/Lobby/WBP_Lobby.WBP_Lobby_C|GetWBP_ColorPicker (Variables|/Game/Frogger/Art/UI/Lobby/BP_LobbyHUD.BP_LobbyHUD_C|GetWBP_Lobby _asbp_lobby_hud))
    (:Is%20Valid
      (Default|UpdateAvailability (Variables|/Game/Frogger/Art/UI/Lobby/WBP_Lobby.WBP_Lobby_C|GetWBP_ColorPicker (Variables|/Game/Frogger/Art/UI/Lobby/BP_LobbyHUD.BP_LobbyHUD_C|GetWBP_Lobby _asbp_lobby_hud)) BlockedColors))))

(event Custom|Multicast_LogEvent
  (params (PlayerName :type Text) (LogType :type E_LogType%20Enum :default "NewEnumerator0"))
  (Default|CallOnLogEvent PlayerName LogType))

(event Custom|Multicast_UpdatePlayerStatus
  (params (NumPlayers :type Integer) (NumReady :type Integer) (OnLogin :type Boolean))
  (Default|CallOnUpdatePlayerStatus (Math|Integer|SelectInt (Variables|Default|GetNumReady) NumReady OnLogin) NumPlayers))

(event Custom|RequestPlayerName
  (params (PlayerState :type BP%20Frogger%20Player%20State%20Object%20Reference))
  (bind _asbp_frogger_player_controller (Utilities|Casting|CastToBP_FroggerPlayerController (Game|GetPlayerController PlayerState)))
  (Default|ClientPlayerStateRequestName _asbp_frogger_player_controller))

(event Custom|StartMatch
  (Networking|SwitchHasAuthority
    (:Authority
      (Development|PrintString "Server Travel!!!")
      (Class|FroggerGameState|TraveltoGame))))

(event Custom|Multicast_StartMatch
  (Networking|SwitchHasAuthority
    (:Authority
      (Game|OpenLevel(byObjectReference) "/Game/Frogger/Maps/GridMap.GridMap" true "listen")
      (Utilities|FlowControl|Delay 1.0)
      (CallFunction|MulticastStartMatch))
    (:Remote
      (Development|ExecuteConsoleCommand (Utilities|String|ToString(Text) (Utilities|Text|FormatText "open {ip}" (Variables|/Game/Frogger/Core/BP_GameInstance.BP_GameInstance_C|GetServerIp (CallFunction|GetGameInstance)))) 0))))

(fn ConstructionScript)