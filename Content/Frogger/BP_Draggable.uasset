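; Frogger component that detects when its owning actor lands on a moving platform, apparently meant to let that platform carry it along.
; After a move, a downward line trace looks for an actor with an InterpToMovement component, then stores it as the bound platform and sets a dragging flag.
; The flag is never cleared here, and the position-following logic is unfinished and unconnected.
; The trace still draws and prints debug output.
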(event Custom|BP_AfterMove
  (bind (_onground _platform) (CallFunction|CheckGround))
  (if _onground
    (Variables|Default|SetBoundPlatform _platform)
    (Variables|Default|SetDragging true)))

(fn CheckGround
  (bind _returnvalue (Components|GetOwner))
  (bind _returnvalue_2 (Transformation|GetActorLocation _returnvalue))
  (bind (_outhit _returnvalue_3) (Collision|LineTraceForObjects _returnvalue_2 (+ _returnvalue_2 "0.000000,0.000000,-300.000000") (Variables|Default|GetObject%20Types) false 0 "ForDuration" true "(R=1.000000,G=0.000000,B=0.000000,A=1.000000)" "(R=0.000000,G=1.000000,B=0.000000,A=1.000000)" 1e+01))
  (if _returnvalue_3
    (Utilities|IsValid (Actor|GetComponentbyClass (.HitActor (Collision|BreakHitResult _outhit)) "/Script/Engine.InterpToMovementComponent")
      (:Is%20Valid
        (Development|PrintString (Utilities|GetDisplayName (Actor|GetComponentbyClass (.HitActor (Collision|BreakHitResult _outhit)) "/Script/Engine.InterpToMovementComponent")))
        (return true (Components|GetOwner (Actor|GetComponentbyClass (.HitActor (Collision|BreakHitResult _outhit)) "/Script/Engine.InterpToMovementComponent"))))
      (:Is%20Not%20Valid
        _)))
  (return false 0))