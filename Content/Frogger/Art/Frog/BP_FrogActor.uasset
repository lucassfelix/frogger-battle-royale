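; BP_FrogActor is a frog actor for the Frogger game that displays a player color on its mesh and tracker widget.
; On BeginPlay it applies the first player color via SetPlayerColor, which sets "Skin Color" on a dynamic material instance and passes the color to WBP_PlayerTracker.
; BindToColorPicker binds an event to each color sample's color-changed callback, printing each index as it goes.
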(event EventBeginPlay
  (CallFunction|SetPlayerColor (Utilities|Array|Get(acopy) (CallFunction|GetPlayerColorsArray))))

(fn ConstructionScript)

(fn SetPlayerColor
  (params (PlayerColor :type Linear%20Color%20Structure))
  (bind _staticmesh (Variables|Default|GetStaticMesh))
  (bind _returnvalue (Rendering|Material|CreateDynamicMaterialInstance _staticmesh 0 (Rendering|Material|GetMaterial _staticmesh 0) "None" :!class /Script/Engine.PrimitiveComponent))
  (Rendering|Material|SetVectorParameterValue _returnvalue "Skin Color" PlayerColor :!class /Script/Engine.MaterialInstanceDynamic)
  (bind _aswbp_player_tracker (Utilities|Casting|CastToWBP_PlayerTracker (UserInterface|GetUserWidgetObject (Variables|Default|GetPlayerTracker))))
  (Default|SetPlayerColor _aswbp_player_tracker PlayerColor))

(fn BindtoColorPicker
  (params (ColorPicker :type WBP%20Color%20Picker%20Object%20Reference))
  (bind _samples (Default|GetAllColorSamples ColorPicker))
  (for (_array_element _array_index) _samples
    (Development|PrintString (Utilities|String|ToString(Integer) _array_index))
    (bind _aswbp_color_sample (Utilities|Casting|CastToWBP_ColorSample _array_element))
    (EventDispatchers|BindEventtoOnColorChanged _aswbp_color_sample (EventDispatchers|CreateEvent :!event SetPlayerColor))))